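; Quest component that holds a player's or actor's active quests and tracks their objective progress.
; On BeginPlay it binds to the game state's gameplay objective event and advances matching objectives by type and target ID.
; Progress is clamped, written back into the runtime struct array, and fires progress and completion events.
; AddQuest builds runtime entries from quest definitions, rejecting duplicate IDs and broadcasting quest start.
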(event `self.ReceiveBeginPlay`
  (bind _asbp_quest_game_state (cast `/Game/QuestsGame/Blueprints/Game_State/BP_QuestGameState` (`GameplayStatics.GetGameState`)))
  (add `/Game/QuestsGame/Blueprints/Game_State/BP_QuestGameState.OnGameplayObjectiveEvent` _asbp_quest_game_state (delegate `HandleGameplayObjective`)))

(event `HandleGameplayObjective`
  (params (ObjectiveType :type "/Game/QuestsGame/Blueprints/Enum/E_QuestObjectiveType Enum" :default "NewEnumerator0") (TargetID :type Name) (Amount :type Integer))
  (for (_array_element _array_index) (`self.ActiveQuests`)
    (bind (_questid _questdefinition _objectives _isactive _iscompleted) (break `/Game/QuestsGame/Blueprints/Structure/ST_QuestRuntime` _array_element))
    (if (and _isactive (not _iscompleted))
      (for (_array_element_2 _array_index_2) _objectives
        (bind (_objectiveid _objectivetype _targetid) (break `/Game/QuestsGame/Blueprints/Structure/ST_QuestObjective` _array_element_2))
        (if (and (`|EnumEquality` ObjectiveType _objectivetype) (== _targetid TargetID))
          (`self.UpdateObjectiveProgress` _array_index _array_index_2 Amount))))))

(fn `AddQuest`
  (params (QuestDefinition :type "/Game/QuestsGame/Blueprints/Data_Asset/PDA_QuestDefinition Object Reference"))
  (locals (QuestRuntime :type "/Game/QuestsGame/Blueprints/Structure/ST_QuestRuntime Structure"))
  (bind _questid (`/Game/QuestsGame/Blueprints/Data_Asset/PDA_QuestDefinition.QuestID` QuestDefinition))
  (`/Engine/EditorBlueprintResources/StandardMacros.IsValid` QuestDefinition
    (:`Is Valid`
      (bind _found (`self.FindQuestByID` _questid))
      (if _found
        (`KismetSystemLibrary.PrintString` "Quest duplicada")
        (else
          (bind _output_get (set `local.QuestRuntime` (make `/Game/QuestsGame/Blueprints/Structure/ST_QuestRuntime` _questid QuestDefinition (`/Game/QuestsGame/Blueprints/Data_Asset/PDA_QuestDefinition.Objectives` QuestDefinition) true)))
          (`KismetArrayLibrary.Array_Add` (`self.ActiveQuests`) _output_get)
          (`self.OnQuestStarted` _output_get))))))

(fn `CheckQuestCompleted`
  (params (QuestIndex :type Integer))
  (returns (IsCompleted :type Boolean))
  (locals (AllCompleted :type Boolean :default true))
  (bind _activequests (`self.ActiveQuests`))
  (bind _output (`|GetArrayItem` _activequests QuestIndex))
  (for _array_element (`.Objectives_14_1B7F1FBF484961253DEFDFB8A62771EF` (break `/Game/QuestsGame/Blueprints/Structure/ST_QuestRuntime` _output))
    (bind (_objectiveid _objectivetype _targetid _requiredamount _currentamount) (break `/Game/QuestsGame/Blueprints/Structure/ST_QuestObjective` _array_element))
    (if (< _currentamount _requiredamount)
      (set `local.AllCompleted` false)
      (break)))
  (if (`local.AllCompleted`)
    (bind _structout (setmembers `/Game/QuestsGame/Blueprints/Structure/ST_QuestRuntime` :`StructRef` _output :`IsActive` false :`IsCompleted` true))
    (`KismetArrayLibrary.Array_Set` _activequests QuestIndex _structout)
    (`self.OnQuestCompleted` _structout))
  (return (`local.AllCompleted`)))

(fn `FindQuestByID`
  (params (QuestID :type Name))
  (returns (Found :type Boolean) (QuestData :type "/Game/QuestsGame/Blueprints/Structure/ST_QuestRuntime Structure") (QuestIndex :type Integer))
  (locals (FoundVar :type Boolean :default false) (QuestDataVar :type "/Game/QuestsGame/Blueprints/Structure/ST_QuestRuntime Structure") (QuestIndexVar :type Integer :default 0))
  (for (_array_element _array_index) (`self.ActiveQuests`)
    (if (== QuestID (`.QuestID_11_064849984BD4F598A7D10C8827E7E8A8` (break `/Game/QuestsGame/Blueprints/Structure/ST_QuestRuntime` _array_element)))
      (set `local.FoundVar` true)
      (set `local.QuestDataVar` _array_element)
      (set `local.QuestIndexVar` _array_index)
      (break)
      (else
        (set `local.FoundVar` false)
        (set `local.QuestIndexVar` -1))))
  (return (`local.FoundVar`) (`local.QuestDataVar`) (`local.QuestIndexVar`)))

(fn `UpdateObjectiveProgress`
  (params (QuestIndex :type Integer) (ObjectiveIndex :type Integer) (Amount :type Integer))
  (locals (UpdatedObjective :type "/Game/QuestsGame/Blueprints/Structure/ST_QuestObjective Structure") (QuestObject :type "/Game/QuestsGame/Blueprints/Structure/ST_QuestRuntime Structure") (ObjectiveArray :type "Array of /Game/QuestsGame/Blueprints/Structure/ST_QuestObjective Structure"))
  (bind _output (`|GetArrayItem` (`self.ActiveQuests`) QuestIndex))
  (bind (_questid _questdefinition _objectives) (break `/Game/QuestsGame/Blueprints/Structure/ST_QuestRuntime` _output))
  (bind _output_2 (`|GetArrayItem` _objectives ObjectiveIndex))
  (bind (_objectiveid _objectivetype _targetid _requiredamount _currentamount) (break `/Game/QuestsGame/Blueprints/Structure/ST_QuestObjective` _output_2))
  (bind _output_get (set `local.QuestObject` _output))
  (bind _output_get_2 (set `local.ObjectiveArray` _objectives))
  (bind _structout (setmembers `/Game/QuestsGame/Blueprints/Structure/ST_QuestObjective` :`StructRef` _output_2 :`CurrentAmount` (`KismetMathLibrary.Clamp` (+ _currentamount Amount) 0 _requiredamount)))
  (bind _output_get_3 (set `local.UpdatedObjective` _structout))
  (`KismetArrayLibrary.Array_Set` _output_get_2 ObjectiveIndex _output_get_3)
  (bind _structout_2 (setmembers `/Game/QuestsGame/Blueprints/Structure/ST_QuestRuntime` :`StructRef` _output_get :`Objectives` _output_get_2))
  (`KismetArrayLibrary.Array_Set` (`self.ActiveQuests`) QuestIndex _structout_2)
  (`self.OnQuestProgressChanged` _structout_2)
  (`self.CheckQuestCompleted` QuestIndex))