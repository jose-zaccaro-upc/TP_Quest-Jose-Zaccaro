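; BP_QuestItem_Collect is a quest pickup actor that can be collected only when an active quest needs it.
; On sphere overlap, it searches the overlapping actor's BP_QuestComponent active quests for an objective matching its TargetID.
; A match reports the objective and Amount to BP_QuestGameState, then destroys the item.
; Without a match, it prints a Spanish "cannot take it yet" message.
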(event `self.SphereCollision.OnComponentBeginOverlap`
  (params (OverlappedComponent :type "PrimitiveComponent Object Reference") (OtherActor :type "Actor Object Reference") (OtherComp :type "PrimitiveComponent Object Reference") (OtherBodyIndex :type Integer) (bFromSweep :type Boolean) (SweepResult :type "HitResult Structure (by ref)"))
  (bind _returnvalue (`self.GetComponentByClass` OtherActor "/Game/QuestsGame/Blueprints/Component/BP_QuestComponent.BP_QuestComponent_C"))
  (bind _cantake (`self.CanTake`))
  (`/Engine/EditorBlueprintResources/StandardMacros.IsValid` _returnvalue
    (:`Is Valid`
      (for _array_element (`/Game/QuestsGame/Blueprints/Component/BP_QuestComponent.ActiveQuests` _returnvalue)
        (if (not _cantake)
          (for _array_element_2 (`.Objectives_14_1B7F1FBF484961253DEFDFB8A62771EF` (break `/Game/QuestsGame/Blueprints/Structure/ST_QuestRuntime` _array_element))
            (if (== (`self.TargetID`) (`.TargetID_10_AE45A65541D6C963247031BD83EF6167` (break `/Game/QuestsGame/Blueprints/Structure/ST_QuestObjective` _array_element_2)))
              (set `self.CanTake` true)
              (break)))))
      (if _cantake
        (bind _asbp_quest_game_state (cast `/Game/QuestsGame/Blueprints/Game_State/BP_QuestGameState` (`GameplayStatics.GetGameState`)))
        (`/Game/QuestsGame/Blueprints/Game_State/BP_QuestGameState.ReportGameplayObjective` _asbp_quest_game_state "NewEnumerator1" (`self.TargetID`) (`self.Amount`))
        (`self.K2_DestroyActor`)
        (else
          (`KismetSystemLibrary.PrintString` "No puedes tomarlo aun"))))))

(fn `UserConstructionScript`)