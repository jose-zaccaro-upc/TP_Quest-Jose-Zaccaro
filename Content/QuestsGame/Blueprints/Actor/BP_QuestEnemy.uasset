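; BP_QuestEnemy is an interactable enemy actor that counts as a target for quest objectives.
; Each Interact call removes one point of Life, clamped so it cannot go negative.
; At zero Life, if the interactor has a BP_QuestComponent, it reports one objective count with its TargetID to BP_QuestGameState, then destroys itself.
; Without that component on the interactor, the enemy is neither reported nor destroyed.
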(event `/Game/QuestsGame/Blueprints/Interface/BPI_Interactable.Interact`
  (params (Interactor :type "Actor Object Reference"))
  (bind _output_get (set `self.Life` (`KismetMathLibrary.Clamp` (- (`self.Life`) 1) 0 999)))
  (if (<= _output_get 0)
    (`/Engine/EditorBlueprintResources/StandardMacros.IsValid` (`self.GetComponentByClass` Interactor "/Game/QuestsGame/Blueprints/Component/BP_QuestComponent.BP_QuestComponent_C")
      (:`Is Valid`
        (bind _asbp_quest_game_state (cast `/Game/QuestsGame/Blueprints/Game_State/BP_QuestGameState` (`GameplayStatics.GetGameState`)))
        (`/Game/QuestsGame/Blueprints/Game_State/BP_QuestGameState.ReportGameplayObjective` _asbp_quest_game_state "NewEnumerator0" (`self.TargetID`) 1)
        (`self.K2_DestroyActor`)))))

(fn `UserConstructionScript`)